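; BP_HttpClient is a VaRest-based HTTP client that controls a lamp's power, color and brightness through a web API.
; Each Send function POSTs a request: toggle builds its URL from BaseURL, while color and brightness send JSON to hardcoded ngrok URLs, brightness without an endpoint path.
; Completion handlers report results through OnRequestFinished; the on/off handlers always flag success, while HandleRequestComplete requires a 200 response.
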(event `HandleSendOnCompleted`
  (params (Request :type "VaRestRequestJSON Object Reference"))
  (bind _returnvalue (`VaRestRequestJSON.GetResponseCode` Request))
  (bind _returnvalue_2 (`VaRestRequestJSON.GetResponseContentAsString` Request true))
  (`KismetSystemLibrary.PrintString` (`KismetStringLibrary.Conv_IntToString` _returnvalue))
  (`self.OnRequestFinished` true _returnvalue_2 _returnvalue))

(event `HandleSendOffCompleted`
  (params (Request :type "VaRestRequestJSON Object Reference"))
  (bind _returnvalue (`VaRestRequestJSON.GetResponseContentAsString` Request true))
  (`self.OnRequestFinished` true _returnvalue (`VaRestRequestJSON.GetResponseCode` Request)))

(event `HandleRequestComplete`
  (params (Request :type "VaRestRequestJSON Object Reference"))
  (bind _returnvalue (`VaRestRequestJSON.GetResponseCode` Request))
  (bind _returnvalue_2 (`VaRestRequestJSON.GetResponseContentAsString` Request true))
  (`self.OnRequestFinished` (== _returnvalue 200) _returnvalue_2 _returnvalue))

(fn `SendBrightness `
  (params (Value :type Integer))
  (bind _returnvalue (subsystem `VaRestSubsystem`))
  (bind _returnvalue_2 (`VaRestSubsystem.ConstructVaRestJsonObject` _returnvalue))
  (`VaRestJsonObject.SetNumberField` _returnvalue_2 "value" (`KismetMathLibrary.Conv_IntToDouble` Value))
  (bind _returnvalue_3 (`VaRestSubsystem.ConstructVaRestRequestExt` _returnvalue "POST" "json"))
  (`VaRestRequestJSON.SetURL` _returnvalue_3 "https://intentionally-unvibrating-matias.ngrok-free.dev")
  (`VaRestRequestJSON.SetRequestObject` _returnvalue_3 _returnvalue_2)
  (add `VaRestRequestJSON.OnRequestComplete` _returnvalue_3 (`|CreateDelegate` :!event `HandleRequestComplete`))
  (`VaRestRequestJSON.ExecuteProcessRequest` _returnvalue_3))

(fn `SendColor`
  (params (R :type Integer) (G :type Integer) (B :type Integer))
  (bind _returnvalue (subsystem `VaRestSubsystem`))
  (`KismetSystemLibrary.PrintString` "\"SendColor called\"")
  (bind _returnvalue_2 (`VaRestSubsystem.ConstructVaRestJsonObject` _returnvalue))
  (`VaRestJsonObject.SetIntegerField` _returnvalue_2 "r" R)
  (`VaRestJsonObject.SetIntegerField` _returnvalue_2 "g" G)
  (`VaRestJsonObject.SetIntegerField` _returnvalue_2 "b" B)
  (bind _returnvalue_3 (`VaRestSubsystem.ConstructVaRestRequestExt` _returnvalue "POST" "json"))
  (`VaRestRequestJSON.SetURL` _returnvalue_3 "https://intentionally-unvibrating-matias.ngrok-free.dev/lamp/color_rgb")
  (`VaRestRequestJSON.SetRequestObject` _returnvalue_3 _returnvalue_2)
  (add `VaRestRequestJSON.OnRequestComplete` _returnvalue_3 (`|CreateDelegate` :!event `HandleRequestComplete`))
  (`VaRestRequestJSON.ExecuteProcessRequest` _returnvalue_3))

(fn `SendToggle`
  (params (bIsOn :type Boolean))
  (if bIsOn
    (bind _returnvalue (`VaRestSubsystem.ConstructVaRestRequestExt` (subsystem `VaRestSubsystem`) "GET" "x_www_form_urlencoded_url"))
    (`VaRestRequestJSON.SetURL` _returnvalue (`KismetStringLibrary.Concat_StrStr` (`self.BaseURL`) "/lamp/on"))
    (`VaRestRequestJSON.SetVerb` _returnvalue "POST")
    (`VaRestRequestJSON.SetHeader` _returnvalue "Content-Type" "application/json")
    (add `VaRestRequestJSON.OnRequestComplete` _returnvalue (`|CreateDelegate` :!event `HandleSendOnCompleted`))
    (`KismetSystemLibrary.PrintString` "Sending ON request")
    (`VaRestRequestJSON.ExecuteProcessRequest` _returnvalue)
    (else
      (bind _returnvalue_2 (`VaRestSubsystem.ConstructVaRestRequestExt` (subsystem `VaRestSubsystem`) "GET" "x_www_form_urlencoded_url"))
      (`VaRestRequestJSON.SetURL` _returnvalue_2 (`KismetStringLibrary.Concat_StrStr` (`self.BaseURL`) "/lamp/off"))
      (`VaRestRequestJSON.SetVerb` _returnvalue_2 "POST")
      (`VaRestRequestJSON.SetHeader` _returnvalue_2 "Content-Type" "application/json")
      (add `VaRestRequestJSON.OnRequestComplete` _returnvalue_2 (`|CreateDelegate` :!event `HandleSendOffCompleted`))
      (`VaRestRequestJSON.ExecuteProcessRequest` _returnvalue_2))))