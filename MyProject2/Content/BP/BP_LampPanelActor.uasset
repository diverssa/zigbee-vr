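; Actor hosting the WBP_LampPanel widget, bridging its lamp controls to an HTTP client and a referenced in-level lamp.
; Color, brightness and color temperature changes are debounced with restartable timers before sending, while toggles and presets send immediately.
; Toggle and color changes also drive the level lamp.
; Request results set the panel's on, off or failure mode, and received lamp state is forwarded to the widget.
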(event `self.ReceiveBeginPlay`
  (bind _aswbp_lamp_panel (cast `/Game/UI/WBP_LampPanel` (`WidgetComponent.GetUserWidgetObject` (`self.Widget`))))
  (set `self.LampPanelWidgetRef` _aswbp_lamp_panel)
  (add `/Game/BP/BP_HttpClient.OnRequestFinished` (`self.HttpClient`) (`|CreateDelegate` :!event `HandleRequestFinished`))
  (add `/Game/UI/WBP_LampPanel.OnToggleChanged` (`self.LampPanelWidgetRef`) (`|CreateDelegate` :!event `HandleToggle`))
  (add `/Game/UI/WBP_LampPanel.OnColorChanged` (`self.LampPanelWidgetRef`) (`|CreateDelegate` :!event `HandleColorChanged`))
  (add `/Game/UI/WBP_LampPanel.OnIntensityChanged` (`self.LampPanelWidgetRef`) (`|CreateDelegate` :!event `HandleIntensityChanged`))
  (add `/Game/UI/WBP_LampPanel.OnColorTempChanged` (`self.LampPanelWidgetRef`) (`|CreateDelegate` :!event `HandleColorTempChanged`))
  (add `/Game/UI/WBP_LampPanel.OnPresetSelected` (`self.LampPanelWidgetRef`) (`|CreateDelegate` :!event `HandlePresetSelected`))
  (add `/Game/UI/WBP_LampPanel.OnTempPresetSelected` (`self.LampPanelWidgetRef`) (`|CreateDelegate` :!event `HandleTempPresetSelected`))
  (add `/Game/UI/WBP_LampPanel.OnColorLinearChanged` (`self.LampPanelWidgetRef`) (`|CreateDelegate` :!event `HandleColorChangedLinear`))
  (add `/Game/BP/BP_HttpClient.OnStateReceived` (`self.HttpClient`) (`|CreateDelegate` :!event `HandleStateReceived`)))

(event `HandleRequestFinished`
  (params (Success :type Boolean) (ResponseString :type String) (StatusCode :type Integer))
  (if (and (and Success (>= StatusCode 200)) (< StatusCode 300))
    (if (`KismetStringLibrary.EqualEqual_StrStr` (`self.DesiredState`) "ON")
      (`/Game/UI/WBP_LampInteract.Update Mode` (`/Game/UI/WBP_LampPanel.WBP_LampInteract` (`self.LampPanelWidgetRef`)) 1)
      (else
        (`/Game/UI/WBP_LampInteract.Update Mode` (`/Game/UI/WBP_LampPanel.WBP_LampInteract` (`self.LampPanelWidgetRef`)) 0)))
    (else
      (`/Game/UI/WBP_LampInteract.Update Mode` (`/Game/UI/WBP_LampPanel.WBP_LampInteract` (`self.LampPanelWidgetRef`)) 2))))

(event `HandleColorChanged`
  (params (R :type Integer) (G :type Integer) (B :type Integer))
  (`KismetSystemLibrary.PrintString` "HandleColor hit")
  (set `self.PendingR` R)
  (set `self.PendingG` G)
  (set `self.PendingB ` B)
  (`KismetSystemLibrary.K2_ClearAndInvalidateTimerHandle` (`self.ColorDebounceHandle`))
  (bind _returnvalue (`KismetSystemLibrary.K2_SetTimer` null "FireColorRequest" (`self.DebounceDelay `)))
  (set `self.ColorDebounceHandle` _returnvalue))

(event `HandleIntensityChanged`
  (params (Value :type Integer))
  (set `self.PendingIntensity ` (`KismetMathLibrary.Conv_IntToDouble` Value))
  (`KismetSystemLibrary.K2_ClearAndInvalidateTimerHandle` (`self.BrightnessDebounceHandle`))
  (bind _returnvalue (`KismetSystemLibrary.K2_SetTimer` null "FireBrightnessRequest" (`self.DebounceDelay `)))
  (set `self.BrightnessDebounceHandle` _returnvalue))

(event `HandleColorTempChanged`
  (params (Value :type Integer))
  (set `self.PendingColorTemp` Value)
  (`KismetSystemLibrary.K2_ClearAndInvalidateTimerHandle` (`self.ColorTempDebounceHandle `))
  (bind _returnvalue (`KismetSystemLibrary.K2_SetTimer` null "FireColorTempRequest" 0.12))
  (set `self.ColorTempDebounceHandle ` _returnvalue))

(event `HandlePresetSelected`
  (params (R :type Integer) (G :type Integer) (B :type Integer))
  (`/Game/BP/BP_HttpClient.SendColor` (`self.HttpClient`) R G B))

(event `HandleTempPresetSelected`
  (params (Value :type Integer))
  (`/Game/BP/BP_HttpClient.SendColorTemp` (`self.HttpClient`) Value))

(event `HandleStateReceived`
  (params (LampState :type "/Game/BP/ST_LampState Structure"))
  (`/Game/UI/WBP_LampPanel.HandleStateReceived` (`self.LampPanelWidgetRef`) LampState))

(fn `FireBrightnessRequest`
  (`/Game/BP/BP_HttpClient.SendBrightness ` (`self.HttpClient`) (`KismetMathLibrary.FTrunc` (`self.PendingIntensity `))))

(fn `FireColorRequest`
  (bind _pendingr (`self.PendingR`))
  (bind _pendingg (`self.PendingG`))
  (bind _pendingb_ (`self.PendingB `))
  (`KismetSystemLibrary.PrintString` "\"FireColorRequest called")
  (`/Game/BP/BP_HttpClient.SendColor` (`self.HttpClient`) _pendingr _pendingg _pendingb_)
  (`/Game/Assets/Led_Lamp/BP_Led_Lamp.SetLampColor` (`self.LampRef`) (make `LinearColor` (`KismetMathLibrary.Conv_IntToDouble` (/ _pendingr 255)) (`KismetMathLibrary.Conv_IntToDouble` (/ _pendingg 255)) (`KismetMathLibrary.Conv_IntToDouble` (/ _pendingb_ 255)) 1.0)))

(fn `FireColorTempRequest`
  (`/Game/BP/BP_HttpClient.SendColorTemp` (`self.HttpClient`) (`self.PendingColorTemp`)))

(fn `HandleColorChangedLinear`
  (params (Color :type "LinearColor Structure"))
  (`/Engine/EditorBlueprintResources/StandardMacros.IsValid` (`self.LampRef`)
    (:`Is Valid`
      (`/Game/Assets/Led_Lamp/BP_Led_Lamp.SetLampColor` (`self.LampRef`) Color))))

(fn `HandleToggle`
  (params (bIsOn :type Boolean))
  (if bIsOn
    (set `self.DesiredState` "ON")
    (`/Game/BP/BP_HttpClient.SendToggle` (`self.HttpClient`) true)
    (`/Game/BP/BP_HttpClient.RequestLampState` (`self.HttpClient`))
    (else
      (set `self.DesiredState` "OFF")
      (`/Game/BP/BP_HttpClient.SendToggle` (`self.HttpClient`) false)))
  (`/Engine/EditorBlueprintResources/StandardMacros.IsValid` (`self.LampRef`)
    (:`Is Valid`
      (`/Game/Assets/Led_Lamp/BP_Led_Lamp.SetLampEnabled` (`self.LampRef`) bIsOn))))

(fn `UserConstructionScript`)