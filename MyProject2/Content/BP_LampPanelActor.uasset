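; BP_LampPanelActor is an actor that links a lamp control panel widget to an HTTP client for controlling a lamp.
; Widget toggle events send on/off requests immediately, while color changes restart a debounce timer that sends only the latest RGB value.
; Finished requests write the last requested on/off state or an error to the panel's status text.
; FireBrightnessRequest is an empty stub.
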(event `self.ReceiveBeginPlay`
  (bind _aswbp_lamp_panel (cast `/Game/WBP_LampPanel` (`WidgetComponent.GetUserWidgetObject` (`self.Widget`))))
  (set `self.LampPanelWidgetRef` _aswbp_lamp_panel)
  (add `/Game/BP_HttpClient.OnRequestFinished` (`self.HttpClient`) (`|CreateDelegate` :!event `HandleRequestFinished`))
  (add `/Game/WBP_LampPanel.OnToggleChanged` (`self.LampPanelWidgetRef`) (`|CreateDelegate` :!event `HandleToggle`))
  (add `/Game/WBP_LampPanel.OnColorChanged` (`self.LampPanelWidgetRef`) (`|CreateDelegate` :!event `HandleColorChanged`)))

(event `HandleRequestFinished`
  (params (Success :type Boolean) (ResponseString :type String) (StatusCode :type Integer))
  (if (and (and Success (>= StatusCode 200)) (< StatusCode 300))
    (if (`KismetStringLibrary.EqualEqual_StrStr` (`self.DesiredState`) "ON")
      (`/Game/WBP_LampPanel.SetStatusText` (`self.LampPanelWidgetRef`) "Status: ON")
      (else
        (`/Game/WBP_LampPanel.SetStatusText` (`self.LampPanelWidgetRef`) "Status: OFF")))
    (else
      (`/Game/WBP_LampPanel.SetStatusText` (`self.LampPanelWidgetRef`) "Error: request failed"))))

(event `HandleColorChanged`
  (params (R :type Integer) (G :type Integer) (B :type Integer))
  (`KismetSystemLibrary.PrintString` "HandleColor hit")
  (set `self.PendingR` R)
  (set `self.PendingG` G)
  (set `self.PendingB ` B)
  (`KismetSystemLibrary.K2_ClearAndInvalidateTimerHandle` (`self.ColorDebounceHandle`))
  (bind _returnvalue (`KismetSystemLibrary.K2_SetTimer` null "FireColorRequest" (`self.DebounceDelay `)))
  (set `self.ColorDebounceHandle` _returnvalue))

(fn `FireBrightnessRequest`)

(fn `FireColorRequest`
  (`KismetSystemLibrary.PrintString` "\"FireColorRequest called")
  (`/Game/BP_HttpClient.SendColor` (`self.HttpClient`) (`self.PendingR`) (`self.PendingG`) (`self.PendingB `)))

(fn `HandleToggle`
  (params (bIsOn :type Boolean))
  (if bIsOn
    (set `self.DesiredState` "ON")
    (`/Game/BP_HttpClient.SendToggle` (`self.HttpClient`) true)
    (else
      (set `self.DesiredState` "OFF")
      (`/Game/BP_HttpClient.SendToggle` (`self.HttpClient`) false))))

(fn `UserConstructionScript`)