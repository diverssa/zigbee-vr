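; BP_Led_Lamp is an LED lamp actor whose glow can be switched on or off and recolored at runtime.
; On BeginPlay it creates a dynamic instance of MI_GlowLamp on its mesh and sets a near-white starting color.
; SetLampEnabled and SetLampColor store the new state, then call ApplyLampVisuals, which pushes the LightColor and on or off EmissiveStrength parameters to that material instance.
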(event `self.ReceiveBeginPlay`
  (bind _returnvalue (`PrimitiveComponent.CreateDynamicMaterialInstance` (`self.Object_5`) 0 "/Game/Assets/Led_Lamp/MI_GlowLamp.MI_GlowLamp" "None"))
  (set `self.LampMID` _returnvalue)
  (`KismetMathLibrary.LinearColor_Set` (`self.CurrentColor`) (struct :`R` 0.9 :`G` 0.9 :`B` 0.9 :`A` 1.0))
  (`KismetSystemLibrary.PrintString` "Create Dynamic Lamp Material"))

(event `SetLampEnabled`
  (params (bIsOn :type Boolean))
  (set `self.bLampEnabled` bIsOn)
  (`self.ApplyLampVisuals`)
  (`KismetSystemLibrary.PrintString` "LampEnabled"))

(event `SetLampColor`
  (params (NewColor :type "LinearColor Structure"))
  (set `self.CurrentColor` NewColor)
  (`self.ApplyLampVisuals`)
  (`KismetSystemLibrary.PrintString` "Change Lamp Color"))

(event `ApplyLampVisuals`
  (`/Engine/EditorBlueprintResources/StandardMacros.IsValid` (`self.LampMID`)
    (:`Is Valid`
      (`MaterialInstanceDynamic.SetVectorParameterValue` (`self.LampMID`) "LightColor" (`self.CurrentColor`))
      (if (`self.bLampEnabled`)
        (`MaterialInstanceDynamic.SetScalarParameterValue` (`self.LampMID`) "EmissiveStrength" (`self.OnEmissiveStrength`))
        (`KismetSystemLibrary.PrintString` "Change Lamp Color ON")
        (else
          (`MaterialInstanceDynamic.SetScalarParameterValue` (`self.LampMID`) "EmissiveStrength" (`self.OffEmissiveStrength`))
          (`KismetSystemLibrary.PrintString` "Change Lamp Color OFF"))))))

(fn `UserConstructionScript`)